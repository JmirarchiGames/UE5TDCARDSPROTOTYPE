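; Tower defense enemy spawner that starts spawning BP_EnemyPawn1 AI pawns at its Sphere component's location on BeginPlay.
; SpawnEnemy re-calls itself after a short delay, incrementing CurrentAmount after each spawn until it equals MaxAmount.
; The limit is checked after spawning, so one extra pawn spawns, then a longer delay runs with nothing following it.
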(event Custom|SpawnEnemy
  (AI|SpawnAIFromClass "/Game/TD/Enemies/BP_EnemyPawn1.BP_EnemyPawn1_C" 0 (Transformation|GetWorldLocation (Variables|Default|GetSphere)) "0, 0, 0" false 0)
  (if (== (Variables|Default|GetCurrentAmount) (Variables|Default|GetMaxAmount))
    (Utilities|FlowControl|Delay 3e+01)
    (else
      (Variables|Default|SetCurrentAmount (+ (Variables|Default|GetCurrentAmount) 1))
      (Utilities|FlowControl|Delay 1.0)
      (CallFunction|SpawnEnemy))))

(event EventBeginPlay
  (CallFunction|SpawnEnemy))

(fn ConstructionScript)