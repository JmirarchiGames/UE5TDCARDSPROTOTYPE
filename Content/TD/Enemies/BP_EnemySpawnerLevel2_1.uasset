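; Tower defense enemy spawner for level 2 that runs escalating waves of BP_EnemyPawn1.
; SpawnEnemy re-calls itself on a delay, spawning at the Sphere's location until the wave cap, then pauses before starting a larger wave.
; Each new wave updates the WWaveAnnouncer counters and adds currency through BP_TowerSpawn.
; Reaching wave 16 shows W_LevelComplete and pauses the game, without waiting for remaining enemies to die.
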(event Custom|SpawnEnemy
  (bind _sphere (Variables|Default|GetSphere))
  (bind _returnvalue (Transformation|GetWorldLocation _sphere))
  (AI|SpawnAIFromClass "/Game/TD/Enemies/BP_EnemyPawn1.BP_EnemyPawn1_C" 0 (Math|Vector|MakeVector (.x _returnvalue) (.y _returnvalue) (.z _returnvalue)) "0, 0, 0" false 0)
  (if (== (Variables|Default|GetCurrentEnemyAmount) (Variables|Default|GetMaxEnemyAmount))
    ;[1 1 1] debug wave announcer
    (Development|PrintString "NEXT WAVE STARTING!")
    (Utilities|FlowControl|Delay 1e+01)
    (Development|PrintString "NEXT WAVE BEGAN!")
    (Variables|Default|SetCurrentWaveNumber (+ (Variables|Default|GetCurrentWaveNumber) 1))
    ;[1 1 1] Updating Wave Announcer Widget
    (bind _foundwidgets (Widget|GetAllWidgetsOfClass "/Game/TD/W-WaveAnnouncer.W-WaveAnnouncer_C" true))
    (Rendering|Components|TextRender|SetText (Variables|/Game/TD/W-WaveAnnouncer.W-WaveAnnouncer_C|GetTXT_WaveCounter (Utilities|Array|Get(acopy) _foundwidgets)) (Utilities|Text|ToText(Integer) (Variables|Default|GetCurrentWaveNumber)))
    (Variables|Default|SetCurrentEnemyAmount 0)
    (Variables|Default|SetMaxEnemyAmount (+ (Variables|Default|GetMaxEnemyAmount) 5))
    ;[1 1 1] Adds currency after each wave
    (bind _outactors (Actor|GetAllActorsOfClass "/Game/TD/BP_TowerSpawn.BP_TowerSpawn_C"))
    (Default|AddCurrency (Utilities|Array|Get(acopy) _outactors) 5)
    (CallFunction|SpawnEnemy)
    (if (>= (Variables|Default|GetCurrentWaveNumber) 16)
      (CallFunction|LevelComplete))
    (else
      (Variables|Default|SetCurrentEnemyAmount (+ (Variables|Default|GetCurrentEnemyAmount) 1))
      (Utilities|FlowControl|Delay 2.0)
      (CallFunction|SpawnEnemy)
      (bind _foundwidgets_2 (Widget|GetAllWidgetsOfClass "/Game/TD/W-WaveAnnouncer.W-WaveAnnouncer_C" true))
      (Variables|/Script/UMG.TextBlock|SetText (Variables|/Game/TD/W-WaveAnnouncer.W-WaveAnnouncer_C|GetTXT_EnemyCounter (Utilities|Array|Get(acopy) _foundwidgets_2)) (Utilities|Text|ToText(Integer) (Variables|Default|GetCurrentEnemyAmount))))))

(event Custom|LevelComplete
  ;[1 1 1] Opens Level Complete Widget
  (bind _returnvalue (UserInterface|CreateWidget "/Game/TD/W_LevelComplete.W_LevelComplete_C"))
  (UserInterface|Viewport|AddtoViewport _returnvalue 0)
  (Variables|/Script/Engine.PlayerController|SetbShowMouseCursor (Game|GetPlayerController 0) true)
  (Game|SetGamePaused true))

(event EventBeginPlay
  (Variables|Default|SetCurrentWaveNumber 1)
  (Utilities|FlowControl|Delay 2.0)
  (CallFunction|SpawnEnemy)
  (bind _returnvalue (UserInterface|CreateWidget "/Game/TD/W-WaveAnnouncer.W-WaveAnnouncer_C"))
  (bind _output_get (Variables|Default|SetWaveAnnouncerUI _returnvalue))
  (UserInterface|Viewport|AddtoViewport _output_get 0))

(event EventTick
  (params (DeltaSeconds :type Float%20%28single-precision%29)))

(fn ConstructionScript)