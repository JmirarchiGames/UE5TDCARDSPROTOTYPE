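; BP_EnemyPawn1 is a tower-defense enemy that walks to BP_Goal by reissuing AI MoveTo every Tick.
; It exposes health and damage functions that forward to BPCDamageSystemComponent, while Heal is a stub returning zero.
; A W_HealthBar widget is created on BeginPlay with the pawn as its damageable actor.
; The component's death event awards currency through the first BP_TowerSpawn and destroys the pawn; damage responses are only logged.
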(event Custom|MoveTo
  (bind _returnvalue (Actor|GetActorOfClass "/Game/TD/BP_Goal.BP_Goal_C"))
  (AI|AIMoveTo self (Transformation|GetActorLocation _returnvalue) 0 5.0 false))

(event Custom|Death
  (bind _outactors (Actor|GetAllActorsOfClass "/Game/TD/BP_TowerSpawn.BP_TowerSpawn_C"))
  (Default|AddCurrency (Utilities|Array|Get(acopy) _outactors) 5)
  (Actor|DestroyActor))

(event Custom|DamageResponse
  (params (DamageResponse :type ENUM_DamageResponse%20Enum :default "NewEnumerator0"))
  (Development|PrintString (Utilities|String|EnumtoString DamageResponse) false))

(event EventBeginPlay
  (bind _returnvalue (UserInterface|CreateWidget "/Game/TD/DamageSystem/W_HealthBar.W_HealthBar_C" 0 self))
  (UserInterface|SetWidget (Variables|Default|GetWidget) _returnvalue))

(event Collision|EventActorBeginOverlap
  (params (OtherActor :type Actor%20Object%20Reference)))

(event EventTick
  (params (DeltaSeconds :type Float%20%28single-precision%29))
  (CallFunction|Moveto))

(fn ConstructionScript
  (bind _bpc_damagesystemcomponent (Variables|Default|GetBPC_DamageSystemComponent))
  (EventDispatchers|BindEventtoOnDeath _bpc_damagesystemcomponent (EventDispatchers|CreateEvent :!event Custom|Death))
  (EventDispatchers|BindEventtoOnDamageResponse _bpc_damagesystemcomponent (EventDispatchers|CreateEvent :!event Custom|DamageResponse)))

(fn GetCurrentHealth
  (return (Variables|/Game/TD/DamageSystem/BPC_DamageSystemComponent.BPC_DamageSystemComponent_C|GetHealth (Variables|Default|GetBPC_DamageSystemComponent))))

(fn GetMaxHealth
  (return (Variables|/Game/TD/DamageSystem/BPC_DamageSystemComponent.BPC_DamageSystemComponent_C|GetMaxHealth (Variables|Default|GetBPC_DamageSystemComponent))))

(fn Heal
  (params (Heal :type Float%20%28double-precision%29))
  (return 0.0))

(fn TakeDamage
  (params (DamageInfo :type STRUCT%20Damage%20Info%20Structure))
  (bind _wasdamaged_ (Default|TakeDamage (Variables|Default|GetBPC_DamageSystemComponent) DamageInfo))
  (return _wasdamaged_))