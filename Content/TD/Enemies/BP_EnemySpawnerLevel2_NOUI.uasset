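; Tower defense enemy spawner for level 2 that runs timed waves of BP_EnemyPawn1 at its sphere's location, without creating its own announcer UI.
; SpawnEnemy re-calls itself on delays; each full wave pauses, updates an existing announcer widget, raises the enemy cap and awards tower currency.
; HighScore resets before comparison, so every wave overwrites the saved score with the current wave number.
; Reaching wave 16 shows the level-complete widget and pauses the game.
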(event Custom|SpawnEnemy
  (bind _sphere (Variables|Default|GetSphere))
  (bind _slotname (Variables|Default|GetSlotName))
  (bind _returnvalue (Transformation|GetWorldLocation _sphere))
  (AI|SpawnAIFromClass "/Game/TD/Enemies/BP_EnemyPawn1.BP_EnemyPawn1_C" 0 (Math|Vector|MakeVector (.x _returnvalue) (.y _returnvalue) (.z _returnvalue)) "0, 0, 0" false 0)
  (if (== (Variables|Default|GetCurrentEnemyAmount) (Variables|Default|GetMaxEnemyAmount))
    ;[1 1 1] debug wave announcer
    (Development|PrintString "NEXT WAVE STARTING!")
    (Utilities|FlowControl|Delay 1e+01)
    (Development|PrintString "NEXT WAVE BEGAN!")
    (Variables|Default|SetCurrentWaveNumber (+ (Variables|Default|GetCurrentWaveNumber) 1))
    ;[1 1 1] Updating Wave Announcer Widget
    (bind _foundwidgets (Widget|GetAllWidgetsOfClass "/Game/TD/W-WaveAnnouncer.W-WaveAnnouncer_C" true))
    (Rendering|Components|TextRender|SetText (Variables|/Game/TD/W-WaveAnnouncer.W-WaveAnnouncer_C|GetTXT_WaveCounter (Utilities|Array|Get(acopy) _foundwidgets)) (Utilities|Text|ToText(Integer) (Variables|Default|GetCurrentWaveNumber)))
    ;[1 1 1] High Score
    (Variables|Default|SetHighScore 0)
    (if (>= (Variables|Default|GetCurrentWaveNumber) (Variables|Default|GetHighScore))
      (bind _output_get (Variables|Default|SetHighScore (Variables|Default|GetCurrentWaveNumber)))
      (bind _returnvalue_2 (SaveGame|DoesSaveGameExist (Variables|Default|GetSlotName)))
      (if _returnvalue_2
        (bind _returnvalue_3 (SaveGame|LoadGamefromSlot (Variables|Default|GetSlotName)))
        (bind _output_get_2 (Variables|Default|SetSaverSubClass _returnvalue_3))
        (bind _asbp_save_game_hs (Utilities|Casting|CastToBP_SaveGameHS _output_get_2))
        (Variables|/Game/TD/SaveGame/BP_SaveGameHS.BP_SaveGameHS_C|SetHighScore _asbp_save_game_hs _output_get)
        (SaveGame|SaveGametoSlot (Variables|Default|GetSaverSubClass) _slotname)
        (else
          (bind _returnvalue_4 (SaveGame|CreateSaveGameObject "/Game/TD/SaveGame/BP_SaveGameHS.BP_SaveGameHS_C"))
          (bind _output_get_3 (Variables|Default|SetSaverSubClass _returnvalue_4))
          (bind _asbp_save_game_hs_2 (Utilities|Casting|CastToBP_SaveGameHS _output_get_3))
          (Variables|/Game/TD/SaveGame/BP_SaveGameHS.BP_SaveGameHS_C|SetHighScore _asbp_save_game_hs_2 _output_get)
          (SaveGame|SaveGametoSlot (Variables|Default|GetSaverSubClass) _slotname))))
    (Variables|Default|SetCurrentEnemyAmount 0)
    (Variables|Default|SetMaxEnemyAmount (+ (Variables|Default|GetMaxEnemyAmount) 5))
    ;[1 1 1] Adds currency after each wave
    (bind _outactors (Actor|GetAllActorsOfClass "/Game/TD/BP_TowerSpawn.BP_TowerSpawn_C"))
    (Default|AddCurrency (Utilities|Array|Get(acopy) _outactors) 5)
    (CallFunction|SpawnEnemy)
    (if (>= (Variables|Default|GetCurrentWaveNumber) 16)
      (CallFunction|LevelComplete))
    (else
      (Variables|Default|SetCurrentEnemyAmount (+ (Variables|Default|GetCurrentEnemyAmount) 1))
      (Utilities|FlowControl|Delay 1.0)
      (CallFunction|SpawnEnemy))))

(event Custom|LevelComplete
  ;[1 1 1] Opens Level Complete Widget
  (bind _returnvalue (UserInterface|CreateWidget "/Game/TD/W_LevelComplete.W_LevelComplete_C"))
  (UserInterface|Viewport|AddtoViewport _returnvalue 0)
  (Variables|/Script/Engine.PlayerController|SetbShowMouseCursor (Game|GetPlayerController 0) true)
  (Game|SetGamePaused true))

(event EventBeginPlay
  ;[1 1 1] Begin Play
  (Variables|Default|SetCurrentWaveNumber 1)
  (Utilities|FlowControl|Delay 2.0)
  (CallFunction|SpawnEnemy))

(event EventTick
  (params (DeltaSeconds :type Float%20%28single-precision%29)))

(fn ConstructionScript)