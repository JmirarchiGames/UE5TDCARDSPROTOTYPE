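; Demo character Blueprint for prototyping pinch-to-zoom on a spring arm camera, still unfinished.
; The IA_CameraZoom input only prints the current touch distance.
; GetTouchDistance measures the gap between two touches, substituting the mouse position's vector length on Windows.
; The Pinch Camera Zoom macro captures starting distance and arm length, but its delta is unused and the arm length setter never runs.
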(event Input|EnhancedActionEvents|EnhancedInputActionIA_CameraZoom
  (params (ActionValue :type Boolean) (ElapsedSeconds :type Float%20%28double-precision%29) (TriggeredSeconds :type Float%20%28double-precision%29) (InputAction :type Input%20Action%20Object%20Reference :default "/Game/TD/Input/MobileZoom/IA_CameraZoom.IA_CameraZoom"))
  (Development|PrintString (Utilities|String|ToString(Float) (CallFunction|GetTouchDistance))))

(fn ConstructionScript)

(fn GetTouchDistance
  (bind _asplayer_controller (Utilities|Casting|CastToPlayerController (Game|GetPlayerController 0)))
  (return (Math|Vector2D|Vector2DLength (select (Utilities|Enum|Equal(Enum) (Game|GetPlatformName) "Windows") (Math|Vector2D|MakeVector2D (.LocationX (Game|Player|GetMousePosition _asplayer_controller)) (.LocationY (Game|Player|GetMousePosition _asplayer_controller))) (- (Math|Vector2D|MakeVector2D (.LocationX (Class|PlayerController|GetInputTouchState _asplayer_controller "Touch1")) (.LocationY (Class|PlayerController|GetInputTouchState _asplayer_controller "Touch1"))) (Math|Vector2D|MakeVector2D (.LocationX (Class|PlayerController|GetInputTouchState _asplayer_controller "Touch2")) (.LocationY (Class|PlayerController|GetInputTouchState _asplayer_controller "Touch2"))))))))