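; Player controller for the tower defense game that shows turret range and opens the pause menu.
; While the upgrade menu is open, Tick draws a debug sphere around the last selected turret at its range, or logs a message if that actor is invalid.
; Pressing P pauses the game, shows the cursor, removes any existing top-level pause menu widgets and adds a fresh one to the viewport.
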(event EventBeginPlay)

(event EventTick
  (params (DeltaSeconds :type Float%20%28single-precision%29))
  (bind _lastselectedactor (Variables|Default|GetLastSelectedActor))
  ;[1 1 1] drawing range of the last selected turret.
  (if (Variables|Default|GetUpgradeMenuOpen?)
    (Utilities|IsValid _lastselectedactor
      (:Is%20Valid
        (Rendering|Debug|DrawDebugSphere (Transformation|GetActorLocation _lastselectedactor) (Variables|Default|GetLastSelectedTurretRange) 50 "(R=0.322894,G=0.075281,B=0.414931,A=1.000000)" 0.1 1.0))
      (:Is%20Not%20Valid
        (Development|PrintString "LastSelectedActor is Invalid!" false)))))

(event Input|KeyboardEvents|P
  (params (Key :type Key%20Structure :default "None"))
  (:Pressed
    (Game|SetGamePaused true)
    (Variables|Default|SetbShowMouseCursor true)
    (bind _foundwidgets (Widget|GetAllWidgetsOfClass "/Game/TD/W-PauseMenu.W-PauseMenu_C" true))
    (for _array_element _foundwidgets
      (Widget|RemovefromParent _array_element))
    (bind _returnvalue (UserInterface|CreateWidget "/Game/TD/W-PauseMenu.W-PauseMenu_C"))
    (UserInterface|Viewport|AddtoViewport _returnvalue 0)))

(fn ConstructionScript)