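; Tower-defense build spot: a clickable plane that opens a tower selection menu.
; Hovering swaps the plane's material, and clicking with Tower true replaces any open W_TowerList with a new one that references this spawn, then hides the plane.
; Each instance also adds a W_Currency widget on BeginPlay and keeps its own Currency value, changed through add and remove events.
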(event OnBeginCursorOver(Plane)
  (params (TouchedComponent :type Primitive%20Component%20Object%20Reference))
  (Rendering|Material|SetMaterial (Variables|Default|GetPlane) 0 "/Game/ImportMeshes/stylized-turrets-pack/source/Black.Black"))

(event OnEndCursorOver(Plane)
  (params (TouchedComponent :type Primitive%20Component%20Object%20Reference))
  (Rendering|Material|SetMaterial (Variables|Default|GetPlane) 0 "/Engine/MapTemplates/Materials/BasicAsset01.BasicAsset01"))

(event OnClicked(Plane)
  (params (TouchedComponent :type Primitive%20Component%20Object%20Reference) (ButtonPressed :type Key%20Structure :default "None"))
  (if (Variables|Default|GetTower?)
    (Rendering|Material|SetMaterial (Variables|Default|GetPlane) 0 0)
    (bind _foundwidgets (Widget|GetAllWidgetsOfClass "/Game/TD/W_TowerList.W_TowerList_C" true))
    (for _array_element _foundwidgets
      (Widget|RemovefromParent _array_element))
    (bind _returnvalue (UserInterface|CreateWidget "/Game/TD/W_TowerList.W_TowerList_C"))
    (UserInterface|Viewport|AddtoViewport _returnvalue 0)
    (Variables|/Game/TD/W_TowerList.W_TowerList_C|SetTowerSpawn _returnvalue self)
    (Rendering|SetVisibility (Variables|Default|GetPlane) false false)
    (else
      (Rendering|Material|SetMaterial (Variables|Default|GetPlane) 0 0))))

(event OnReleased(Plane)
  (params (TouchedComponent :type Primitive%20Component%20Object%20Reference) (ButtonReleased :type Key%20Structure :default "None"))
  (Rendering|Material|SetMaterial (Variables|Default|GetPlane) 0 "/Engine/MapTemplates/Materials/BasicAsset01.BasicAsset01"))

(event Custom|AddCurrency
  (params (Added%20Currency :type Integer))
  (Variables|Default|SetCurrency (+ (Variables|Default|GetCurrency) Added%20Currency)))

(event Custom|RemoveCurrency
  (params (Removed%20Currency :type Integer))
  (Variables|Default|SetCurrency (- (Variables|Default|GetCurrency) Removed%20Currency)))

(event EventBeginPlay
  (bind _returnvalue (UserInterface|CreateWidget "/Game/TD/W_Currency.W_Currency_C"))
  (bind _output_get (Variables|Default|SetCurrency_Ref _returnvalue))
  (UserInterface|Viewport|AddtoViewport _output_get 0))

(event Collision|EventActorBeginOverlap
  (params (OtherActor :type Actor%20Object%20Reference)))

(event EventTick
  (params (DeltaSeconds :type Float%20%28single-precision%29)))

(fn ConstructionScript)