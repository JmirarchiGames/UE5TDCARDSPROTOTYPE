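; BP_Ballistic_Mine is a tower-defense mine that explodes shortly after something overlaps its cylinder trigger.
; The overlap, which is not filtered by actor type, turns the RectLight red and starts a short delay.
; The mine then sphere-queries nearby BP_EnemyPawn1 pawns, sends them a damage-struct message, spawns an explosion emitter and destroys itself.
; A Duration-based self-destruct exists but is unconnected, so the mine never expires on its own.
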(event OnComponentBeginOverlap(Cylinder)
  (params (OverlappedComponent :type Primitive%20Component%20Object%20Reference) (OtherActor :type Actor%20Object%20Reference) (OtherComp :type Primitive%20Component%20Object%20Reference) (OtherBodyIndex :type Integer) (bFromSweep :type Boolean) (SweepResult :type Hit%20Result%20Structure%20%28by%20ref%29))
  (bind _defaultsceneroot (Variables|Default|GetDefaultSceneRoot))
  (bind _returnvalue (Transformation|GetWorldTransform _defaultsceneroot))
  (Rendering|Components|Light|SetLightColor (Variables|Default|GetRectLight) "(R=1.000000,G=0.000000,B=0.090672,A=1.000000)" true)
  (Utilities|FlowControl|Delay 0.5)
  (bind _outactors (Collision|SphereOverlapActors (.location _returnvalue) 2e+02 (Utilities|Array|MakeArray "ObjectTypeQuery3") "/Game/TD/Enemies/BP_EnemyPawn1.BP_EnemyPawn1_C"))
  (Class|BPIDamageable|TakeDamage(Message) _outactors (Utilities|Struct|MakeSTRUCT_DamageInfo (Variables|Default|GetDmgAmount) "NewEnumerator2"))
  (Effects|SpawnEmitteratLocation "/Game/FXVarietyPack/Particles/P_ky_explosion.P_ky_explosion" (.location _returnvalue) (.rotation _returnvalue))
  (Actor|DestroyActor))

(event EventBeginPlay
  ;[1 1 1] Duration in seconds (Unconnected)
)

(fn ConstructionScript)