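; BP_Projectile_Slowing is a tower defense projectile that deals area damage and leaves a slowing aura where it hits.
; On collider hit, a sphere overlap finds nearby enemy pawns and sends them a typed damage message.
; A successful message spawns SlowingAura with an ice sound, then destroys the projectile.
; With at least two Elemental traits on the player controller, impacts also have a one-in-ten chance to spawn BP_ElementalStorm.
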(event OnComponentHit(BoxCollider)
  (params (HitComponent :type Primitive%20Component%20Object%20Reference) (OtherActor :type Actor%20Object%20Reference) (OtherComp :type Primitive%20Component%20Object%20Reference) (NormalImpulse :type Vector :default "0, 0, 0") (Hit :type Hit%20Result%20Structure%20%28by%20ref%29))
  (bind _impactpoint (Collision|BreakHitResult Hit))
  (bind _returnvalue (Math|Conversions|ToTransform(Vector) _impactpoint))
  (bind _outactors (Collision|SphereOverlapActors _impactpoint 1.5e+02 (Utilities|Array|MakeArray "ObjectTypeQuery3") "/Game/TD/Enemies/BP_EnemyPawn1.BP_EnemyPawn1_C"))
  (bind _wasdamaged_ (Class|BPIDamageable|TakeDamage(Message) _outactors (Utilities|Struct|MakeSTRUCT_DamageInfo (Variables|Default|GetAmount%20Of%20Damage) "NewEnumerator1")))
  (if _wasdamaged_
    (Game|SpawnActorfromClass "/Game/TD/Projectile/SlowingAura.SlowingAura_C" _returnvalue "Undefined" "MultiplyWithRoot" 0 0)
    (Audio|SpawnSoundatLocation "/Game/Interface_And_Item_Sounds/ImportedOtherSounds/709888__lotteria001__ice-magic-arrow_type-01.709888__lotteria001__ice-magic-arrow_type-01" _impactpoint "0, 0, 0" 0.2 0.8 0.0 0 0)
    ;[1 1 1] Checking how many of tower type
    (bind _asbp_player_controller_tdgame (Utilities|Casting|CastToBP_PlayerControllerTDGAME (Game|GetPlayerController 0)))
    (if (>= (Variables|/Game/TD/BP_PlayerControllerTDGAME.BP_PlayerControllerTDGAME_C|GetTraitCount_Elemental _asbp_player_controller_tdgame) 2)
      (if (== (Math|Random|RandomIntegerinRange 1 10) 1)
        (Game|SpawnActorfromClass "/Game/TD/BP_ElementalStorm.BP_ElementalStorm_C" _returnvalue "Undefined" "MultiplyWithRoot" 0 0)))
    (Actor|DestroyActor self)))

(event EventBeginPlay
  (|CallParentFunction) ; This node is disabled and will not be called.\nDrag off pins to build functionality.
)

(event Collision|EventActorBeginOverlap
  (params (OtherActor :type Actor%20Object%20Reference))
  (|CallParentFunction OtherActor) ; This node is disabled and will not be called.\nDrag off pins to build functionality.
)

(event EventTick
  (params (DeltaSeconds :type Float%20%28single-precision%29))
  (|CallParentFunction DeltaSeconds) ; This node is disabled and will not be called.\nDrag off pins to build functionality.
)

(fn ConstructionScript
  (|CallParentFunction))