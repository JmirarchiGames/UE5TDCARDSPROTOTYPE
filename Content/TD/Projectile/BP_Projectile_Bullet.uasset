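; BP_Projectile_Bullet is a bullet projectile actor that deals damage to the actor it hits.
; On a BoxCollider hit, it sends a TakeDamageMessage to the hit actor with a damage struct holding its damage amount and a fixed type.
; When that call returns true, it spawns a small impact particle and a quiet, pitch-randomized gunshot sound at the impact point, then destroys itself after a short delay.
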(event OnComponentHit(BoxCollider)
  (params (HitComponent :type Primitive%20Component%20Object%20Reference) (OtherActor :type Actor%20Object%20Reference) (OtherComp :type Primitive%20Component%20Object%20Reference) (NormalImpulse :type Vector :default "0, 0, 0") (Hit :type Hit%20Result%20Structure%20%28by%20ref%29))
  (bind (_bblockinghit _binitialoverlap _time _distance _location _impactpoint _normal _impactnormal _physmat _hitactor) (Collision|BreakHitResult Hit))
  (bind _wasdamaged_ (Class|BPIDamageable|TakeDamage(Message) _hitactor (Utilities|Struct|MakeSTRUCT_DamageInfo (Variables|Default|GetAmount%20Of%20Damage) "NewEnumerator2")))
  (if _wasdamaged_
    (Effects|SpawnEmitteratLocation "/Game/FXVarietyPack/Particles/P_ky_hit2.P_ky_hit2" _impactpoint "0, 0, 0" "0.200000,0.200000,0.200000")
    (Audio|SpawnSoundatLocation "/Game/Interface_And_Item_Sounds/ImportedOtherSounds/369528__johandeecke__short-gunshot.369528__johandeecke__short-gunshot" _impactpoint "0, 0, 0" 0.1 (Math|Random|RandomFloatinRange 0.8 1.3) 0.0 0 0)
    (Utilities|FlowControl|Delay 0.25)
    (Actor|DestroyActor self)))

(event EventBeginPlay
  (|CallParentFunction) ; This node is disabled and will not be called.\nDrag off pins to build functionality.
)

(event Collision|EventActorBeginOverlap
  (params (OtherActor :type Actor%20Object%20Reference))
  (|CallParentFunction OtherActor) ; This node is disabled and will not be called.\nDrag off pins to build functionality.
)

(event EventTick
  (params (DeltaSeconds :type Float%20%28single-precision%29))
  (|CallParentFunction DeltaSeconds) ; This node is disabled and will not be called.\nDrag off pins to build functionality.
)

(fn ConstructionScript
  (|CallParentFunction))