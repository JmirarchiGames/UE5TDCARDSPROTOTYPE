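; Magic projectile that deals area damage to enemy pawns where it hits.
; When its box collider hits, a sphere overlap at the impact point gathers nearby BP_EnemyPawn1 actors and sends them a TakeDamageMessage with a damage amount and type struct.
; If that message returns true, it spawns a scaled-down thunder-ball hit particle and destroys itself after a short delay.
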(event OnComponentHit(BoxCollider)
  (params (HitComponent :type Primitive%20Component%20Object%20Reference) (OtherActor :type Actor%20Object%20Reference) (OtherComp :type Primitive%20Component%20Object%20Reference) (NormalImpulse :type Vector :default "0, 0, 0") (Hit :type Hit%20Result%20Structure%20%28by%20ref%29))
  (bind _impactpoint (Collision|BreakHitResult Hit))
  (bind _outactors (Collision|SphereOverlapActors _impactpoint 1e+02 (Utilities|Array|MakeArray "ObjectTypeQuery3") "/Game/TD/Enemies/BP_EnemyPawn1.BP_EnemyPawn1_C"))
  (bind _wasdamaged_ (Class|BPIDamageable|TakeDamage(Message) _outactors (Utilities|Struct|MakeSTRUCT_DamageInfo 3.0 "NewEnumerator1")))
  (if _wasdamaged_
    (Effects|SpawnEmitteratLocation "/Game/FXVarietyPack/Particles/P_ky_ThunderBallHit.P_ky_ThunderBallHit" _impactpoint "0, 0, 0" "0.200000,0.200000,0.200000")
    (Utilities|FlowControl|Delay 0.2)
    (Actor|DestroyActor self)))

(event EventBeginPlay
  (|CallParentFunction) ; This node is disabled and will not be called.\nDrag off pins to build functionality.
)

(event Collision|EventActorBeginOverlap
  (params (OtherActor :type Actor%20Object%20Reference))
  (|CallParentFunction OtherActor) ; This node is disabled and will not be called.\nDrag off pins to build functionality.
)

(event EventTick
  (params (DeltaSeconds :type Float%20%28single-precision%29))
  (|CallParentFunction DeltaSeconds) ; This node is disabled and will not be called.\nDrag off pins to build functionality.
)

(fn ConstructionScript
  (|CallParentFunction))