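; Tower-defense slowing turret that automatically fires BP_Projectile_Slowing at enemy pawns within its sensing range.
; Each tick it selects the nearest enemy with line of sight, rotates its Connector toward it and fires once the fire interval has elapsed and aim is aligned.
; Projectile impacts send typed damage to the hit actor.
; Clicking or touching the tower opens its turret menu and registers it as selected on the player controller.
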(event OnClicked(Box)
  (params (TouchedComponent :type Primitive%20Component%20Object%20Reference) (ButtonPressed :type Key%20Structure :default "None"))
  ;[1 1 1] tower menu
  (bind _returnvalue (UserInterface|CreateWidget "/Game/TD/TowerMenu/TurretMenu_4.TurretMenu_4_C"))
  (UserInterface|Viewport|AddtoViewport _returnvalue 0)
  (bind _asbp_player_controller_tdgame (Utilities|Casting|CastToBP_PlayerControllerTDGAME (Game|GetPlayerController 0))
    (:then
      (Variables|/Game/TD/BP_PlayerControllerTDGAME.BP_PlayerControllerTDGAME_C|SetLastSelectedActor _asbp_player_controller_tdgame self)
      (Variables|/Game/TD/BP_PlayerControllerTDGAME.BP_PlayerControllerTDGAME_C|SetLastSelectedTurretRange _asbp_player_controller_tdgame (Variables|Default|GetTurretSensingRange))
      (Variables|/Game/TD/BP_PlayerControllerTDGAME.BP_PlayerControllerTDGAME_C|SetUpgradeMenuOpen? _asbp_player_controller_tdgame true))
    (:CastFailed
      (Development|PrintString "cast to player controller failed!"))))

(event OnInputTouchBegin(Box)
  (params (FingerIndex :type ETouchIndex%20Enum :default "Touch1") (TouchedComponent :type Primitive%20Component%20Object%20Reference))
  ;[1 1 1] tower menu
  (bind _returnvalue (UserInterface|CreateWidget "/Game/TD/TowerMenu/TurretMenu_4.TurretMenu_4_C"))
  (UserInterface|Viewport|AddtoViewport _returnvalue 0)
  (bind _asbp_player_controller_tdgame (Utilities|Casting|CastToBP_PlayerControllerTDGAME (Game|GetPlayerController 0))
    (:then
      (Variables|/Game/TD/BP_PlayerControllerTDGAME.BP_PlayerControllerTDGAME_C|SetLastSelectedActor _asbp_player_controller_tdgame self)
      (Variables|/Game/TD/BP_PlayerControllerTDGAME.BP_PlayerControllerTDGAME_C|SetLastSelectedTurretRange _asbp_player_controller_tdgame (Variables|Default|GetTurretSensingRange))
      (Variables|/Game/TD/BP_PlayerControllerTDGAME.BP_PlayerControllerTDGAME_C|SetUpgradeMenuOpen? _asbp_player_controller_tdgame true))
    (:CastFailed
      (Development|PrintString "cast to player controller failed!"))))

(event Custom|Fire
  (Variables|Default|SetTimeOfLastFire (Utilities|Time|GetGameTimeinSeconds))
  (Utilities|FlowControl|Sequence
    (:then_0
      (Utilities|FlowControl|DoOnce false :!label _label
        (:Completed
          (bind _returnvalue (Game|SpawnActorfromClass "/Game/TD/Projectile/BP_Projectile_Slowing.BP_Projectile_Slowing_C" (Transformation|GetWorldTransform (Variables|Default|GetFirePoint)) "AlwaysSpawn" "MultiplyWithRoot" self 0))
          (EventDispatchers|BindEventtoOnProjectileImpact _returnvalue (delegate Custom|DamageEnemy))
          (Utilities|FlowControl|Delay 0.1))))
    (:then_1
      (goto _label Reset))))

(event Custom|DamageEnemy
  (params (OtherActor :type Actor%20Object%20Reference) (Hit :type Hit%20Result%20Structure))
  (Class|BPIDamageable|TakeDamage(Message) OtherActor (Utilities|Struct|MakeSTRUCT_DamageInfo (Variables|Default|GetTurretDamage) "NewEnumerator1")))

(event EventBeginPlay)

(event Collision|EventActorBeginOverlap
  (params (OtherActor :type Actor%20Object%20Reference)))

(event EventTick
  (params (DeltaSeconds :type Float%20%28single-precision%29))
  (CallFunction|FindBestTarget)
  (Variables|Default|GetTarget
    (:then
      (CallFunction|UpdateTurretRotation DeltaSeconds)
      (CallFunction|UpdateFire))
    (:else)))

(fn ConstructionScript)

(fn FindBestTarget
  (LocalVariables|SetBestDistance%28local%29 (+ (Variables|Default|GetTurretSensingRange) 1.0))
  (bind _outactors (Collision|SphereOverlapActors (Transformation|GetActorLocation) (Variables|Default|GetTurretSensingRange) (Utilities|Array|MakeArray "ObjectTypeQuery3") "/Game/TD/Enemies/BP_EnemyPawn1.BP_EnemyPawn1_C"))
  ;[1 1 1] Looped
  (for _array_element _outactors
    (bind _output_get (LocalVariables|SetCurrentTarget%28local%29 _array_element))
    (bind _output_get_2 (LocalVariables|SetCurrentDistance%28local%29 (Transformation|GetDistanceTo _output_get self)))
    (if (or (< _output_get_2 (LocalVariables|GetBestDistance%28local%29)) (not (Utilities|IsValid (LocalVariables|GetBestTarget%28local%29))))
      (bind _result (CallFunction|HasLineOfSight (Transformation|GetWorldLocation (Variables|Default|GetFirePoint)) (Transformation|GetActorLocation (LocalVariables|GetCurrentTarget%28local%29)) (Utilities|Array|MakeArray self (LocalVariables|GetCurrentTarget%28local%29))))
      (if _result
        (LocalVariables|SetBestTarget%28local%29 (LocalVariables|GetCurrentTarget%28local%29))
        (LocalVariables|SetBestDistance%28local%29 (LocalVariables|GetCurrentDistance%28local%29)))))
  (Variables|Default|SetTarget (LocalVariables|GetBestTarget%28local%29)))

(fn UpdateTurretRotation
  (params (Delta%20Seconds :type Float%20%28double-precision%29))
  (bind _connector (Variables|Default|GetConnector))
  (Transformation|SetWorldRotation _connector (Class|KismetMathLibrary|RInterptoConstant (Transformation|GetWorldRotation _connector) (Math|Rotator|FindLookatRotation (Transformation|GetWorldLocation _connector) (Transformation|GetActorLocation (Variables|Default|GetTarget))) Delta%20Seconds (Variables|Default|GetInterp%20Speed)) false false))

(fn UpdateFire
  (bind _connector (Variables|Default|GetConnector))
  (if (> (- (Utilities|Time|GetGameTimeinSeconds) (Variables|Default|GetTimeOfLastFire)) (Variables|Default|GetRateOfFire))
    ;[1 1 1] is turret facing target?
    (if (> (Math|Vector|DotProduct (Math|Vector|GetUnitDirection(Vector) (Transformation|GetWorldLocation _connector) (Transformation|GetActorLocation (Variables|Default|GetTarget))) (Math|Vector|GetForwardVector _connector)) 0.99)
      (CallFunction|Fire))))