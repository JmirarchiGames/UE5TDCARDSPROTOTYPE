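; BP_Goal is the tower-defense base actor that loses health as enemies reach it, ending the game at zero.
; BeginPlay fills health and adds a friendly health bar widget that references the goal.
; Box overlaps pass a DoOnce gate, then destroy the other actor, subtracting health only for exact BP_EnemyPawn1 class matches.
; The gate resets until health runs out, when GameOver shows its widget, cursor and pauses.
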(event OnComponentBeginOverlap(Box)
  (params (OverlappedComponent :type Primitive%20Component%20Object%20Reference) (OtherActor :type Actor%20Object%20Reference) (OtherComp :type Primitive%20Component%20Object%20Reference) (OtherBodyIndex :type Integer) (bFromSweep :type Boolean) (SweepResult :type Hit%20Result%20Structure%20%28by%20ref%29))
  (for _array_element (Utilities|Array|MakeArray SweepResult)
    (Utilities|FlowControl|DoOnce false :!label _label
      (:Completed
        (if (== (Utilities|GetClass OtherActor) "/Game/TD/Enemies/BP_EnemyPawn1.BP_EnemyPawn1_C")
          (Variables|Default|SetBaseCurrentHealth (- (Variables|Default|GetBaseCurrentHealth) 1.0))
          (Actor|DestroyActor OtherActor)
          (if (<= (Variables|Default|GetBaseCurrentHealth) 0.0)
            (CallFunction|GameOver)
            (else
              (goto _label Reset)))
          (else
            (Development|PrintString "The  enemy is of the wrong type! no damage was taken by the goal.")
            (Actor|DestroyActor OtherActor)
            (goto _label Reset)))))))

(event Custom|GameOver
  (bind _returnvalue (UserInterface|CreateWidget "/Game/TD/W_GameOver.W_GameOver_C"))
  (UserInterface|Viewport|AddtoViewport _returnvalue 0)
  (Variables|/Script/Engine.PlayerController|SetbShowMouseCursor (Game|GetPlayerController 0) true)
  (Game|SetGamePaused true))

(event Input|EnhancedActionEvents|EnhancedInputActionIA_GameOver
  (params (ActionValue :type Boolean) (ElapsedSeconds :type Float%20%28double-precision%29) (TriggeredSeconds :type Float%20%28double-precision%29) (InputAction :type Input%20Action%20Object%20Reference :default "/Game/TopDown/Input/IA_GameOver.IA_GameOver"))
  (:Started
    (Development|PrintString "Hello")))

(event EventBeginPlay
  (bind _output_get (Variables|Default|SetBaseMaxHealth (Variables|Default|GetBaseMaxHealth)))
  (Variables|Default|SetBaseCurrentHealth _output_get)
  (bind _returnvalue (UserInterface|CreateWidget "/Game/TD/DamageSystem/W_HealthBar_Friendly.W_HealthBar_Friendly_C" 0 self))
  (UserInterface|Viewport|AddtoViewport _returnvalue 0))

(event Collision|EventActorBeginOverlap
  (params (OtherActor :type Actor%20Object%20Reference)))

(fn ConstructionScript)