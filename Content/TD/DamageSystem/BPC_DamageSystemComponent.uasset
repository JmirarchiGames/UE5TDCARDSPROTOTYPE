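; Damage system component that tracks health and death for its owner through a TakeDamage function returning whether damage was applied.
; A macro routes each hit to no damage if already dead, otherwise double, half or normal damage from the vulnerability and resistance flags.
; All damaging branches reduce Health and can set IsDead, but only normal damage calls OnDeath or OnDamageResponse.
; Invincibility is hard-coded off.
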(event EventBeginPlay)

(event EventTick
  (params (DeltaSeconds :type Float%20%28single-precision%29)))

(fn TakeDamage
  (params (DamageInfo :type STRUCT%20Damage%20Info%20Structure))
  (bind (_amountofdamage _damagetype _damageresponse _isvulnerable_ _isresistant_) (Utilities|Struct|BreakSTRUCT_DamageInfo DamageInfo))
  ;[1 1 1] Need to setup Double/half damage functions
  (Utilities|DamageMacro _isvulnerable_ false _isresistant_
    (:NoDamage
      (return false))
    (:NormalDamage
      ;[1 1 1] Normal
      (bind _output_get (Variables|Default|SetHealth (- (Variables|Default|GetHealth) _amountofdamage)))
      (if (<= _output_get 0.0)
        (Variables|Default|SetIsDead? true)
        (Default|CallOnDeath)
        (return true)
        (else
          (Default|CallOnDamageResponse "NewEnumerator0")
          ;[1 1 1] Implelement damage response effect here
          (return true))))
    (:DoubleDamage
      ;[1 1 1] Double
      (bind _output_get_2 (Variables|Default|SetHealth (- (Variables|Default|GetHealth) (* _amountofdamage 2.0))))
      (if (<= _output_get_2 0.0)
        (Variables|Default|SetIsDead? true)
        (return true)
        (else
          (return true))))
    (:HalfDamage
      ;[1 1 1] Half
      (bind _output_get_3 (Variables|Default|SetHealth (- (Variables|Default|GetHealth) (* _amountofdamage 0.5))))
      (if (<= _output_get_3 0.0)
        (Variables|Default|SetIsDead? true)
        (return true)
        (else
          (return true))))))