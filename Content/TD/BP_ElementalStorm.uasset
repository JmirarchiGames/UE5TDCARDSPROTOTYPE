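; BP_ElementalStorm is a short-lived tower-defense storm that damages enemy pawns around it and destroys itself after six seconds.
; BeginPlay plays an attached blizzard sound with random pitch and starts the lifetime delay.
; A hitbox overlap starts a repeating sphere query that sends damage through a TakeDamageMessage call every half second, with ice sounds.
; TornadoMovement is an empty stub, and the random-wander logic is disconnected.
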(event OnComponentBeginOverlap(CylinderHitbox)
  (params (OverlappedComponent :type Primitive%20Component%20Object%20Reference) (OtherActor :type Actor%20Object%20Reference) (OtherComp :type Primitive%20Component%20Object%20Reference) (OtherBodyIndex :type Integer) (bFromSweep :type Boolean) (SweepResult :type Hit%20Result%20Structure%20%28by%20ref%29))
  ;[1 1 1] looping dmg each 0.5 second
  (bind _outactors (Collision|SphereOverlapActors (.location (Transformation|GetWorldTransform (Variables|Default|GetDefaultSceneRoot))) 1.2e+02 (Utilities|Array|MakeArray "ObjectTypeQuery3") "/Game/TD/Enemies/BP_EnemyPawn1.BP_EnemyPawn1_C" :!label _label))
  (bind _wasdamaged_ (Class|BPIDamageable|TakeDamage(Message) _outactors (Utilities|Struct|MakeSTRUCT_DamageInfo 3.0 "NewEnumerator1")))
  (if _wasdamaged_
    (Audio|SpawnSoundAttached "/Game/Interface_And_Item_Sounds/ImportedOtherSounds/536807__egomassive__ice.536807__egomassive__ice" (Variables|Default|GetStorm) "None" "0, 0, 0" "0, 0, 0" "KeepRelativeOffset" false 0.5 (Math|Random|RandomFloatinRange 0.8 1.3) 0.0 0 0))
  (Utilities|FlowControl|Delay 0.5)
  (goto _label))

(event Custom|TornadoMovement)

(event EventBeginPlay
  ;[1 1 1] Duration
  (Audio|SpawnSoundAttached "/Game/Interface_And_Item_Sounds/ImportedOtherSounds/573290__kevp888__210523_1598_fr_blizzard.573290__kevp888__210523_1598_fr_blizzard" (Variables|Default|GetDefaultSceneRoot) "None" "0, 0, 0" "0, 0, 0" "KeepRelativeOffset" true 0.5 (Math|Random|RandomFloatinRange 0.8 1.3) 0.0 0 0)
  (CallFunction|TornadoMovement)
  (Utilities|FlowControl|Delay 6.0)
  (Actor|DestroyActor))

(event EventTick
  (params (DeltaSeconds :type Float%20%28single-precision%29)))

(fn ConstructionScript)