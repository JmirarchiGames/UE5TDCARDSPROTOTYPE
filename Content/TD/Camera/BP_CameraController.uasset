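; Top-down style camera controller for the TD game that pans by touch drag.
; BeginPlay enables cursor and touch events and adds two Enhanced Input mapping contexts.
; IA_Drag records the starting touch, then Tick moves the actor by each frame's Touch1 delta, mapping screen axes to world X/Y.
; Mouse panning is disconnected, and pinch zoom via touch distance and spring arm length is unfinished.
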(event Input|EnhancedActionEvents|EnhancedInputActionIA_CameraZoom
  (params (ActionValue :type Boolean) (ElapsedSeconds :type Float%20%28double-precision%29) (TriggeredSeconds :type Float%20%28double-precision%29) (InputAction :type Input%20Action%20Object%20Reference :default "/Game/TD/MobileZoom/IA_CameraZoom.IA_CameraZoom")))

(event Input|EnhancedActionEvents|EnhancedInputActionIA_Drag
  (params (ActionValue :type Boolean) (ElapsedSeconds :type Float%20%28double-precision%29) (TriggeredSeconds :type Float%20%28double-precision%29) (InputAction :type Input%20Action%20Object%20Reference :default "/Game/TD/Input/IA_Drag.IA_Drag"))
  (bind _returnvalue (Game|GetPlayerController 0))
  (bind (_locationx _locationy) (Class|PlayerController|GetInputTouchState _returnvalue "Touch1"))
  (:Started
    (Variables|Default|SetPreviousTouchLocation (Math|Vector2D|MakeVector2D _locationx _locationy))))

(event EventBeginPlay
  (bind _returnvalue (Game|GetPlayerController 0))
  (Input|SetInputModeGameandUI (Game|GetPlayerController 0) 0 "DoNotLock" false false)
  (Variables|/Script/Engine.PlayerController|SetbShowMouseCursor _returnvalue true)
  (Variables|/Script/Engine.PlayerController|SetbEnableTouchEvents _returnvalue true)
  (bind _asplayer_controller (Utilities|Casting|CastToPlayerController (Pawn|GetController))
    (:then
      (Utilities|IsValid (PlayerController|LocalPlayerSubsystems|GetEnhancedInputLocalPlayerSubsystem _asplayer_controller)
        (:Is%20Valid
          (Input|AddMappingContext (PlayerController|LocalPlayerSubsystems|GetEnhancedInputLocalPlayerSubsystem _asplayer_controller) "/Game/TD/Input/IM_Game.IM_Game" 0 "(bIgnoreAllPressedKeysUntilRelease=True,bForceImmediately=False,bNotifyUserSettings=False)")
          (Input|AddMappingContext (PlayerController|LocalPlayerSubsystems|GetEnhancedInputLocalPlayerSubsystem _asplayer_controller) "/Game/TopDown/Input/IMC_Default.IMC_Default" 0 "(bIgnoreAllPressedKeysUntilRelease=True,bForceImmediately=False,bNotifyUserSettings=False)"))
        (:Is%20Not%20Valid
          (Development|PrintString "BP_CameraController INVALID NODE FAILED!"))))
    (:CastFailed
      (Development|PrintString "BP_CameraController CAST FAILED!"))))

(event EventTick
  (params (DeltaSeconds :type Float%20%28single-precision%29))
  (bind _returnvalue (Game|GetPlayerController 0))
  (bind (_locationx _locationy _biscurrentlypressed) (Class|PlayerController|GetInputTouchState _returnvalue "Touch1"))
  (if _biscurrentlypressed
    (Variables|Default|SetNewTouchLoacation (Math|Vector2D|MakeVector2D _locationx _locationy))
    (Class|Actor|AddActorWorldTransform (Math|Transform|MakeTransform (Math|Vector|MakeVector (.y (- (Variables|Default|GetNewTouchLoacation) (Variables|Default|GetPreviousTouchLocation))) (* (.x (- (Variables|Default|GetNewTouchLoacation) (Variables|Default|GetPreviousTouchLocation))) -1.0) 0.0) "0, 0, 0" "1.000000,1.000000,1.000000") false false)
    (Variables|Default|SetPreviousTouchLocation (Variables|Default|GetNewTouchLoacation))))

(fn ConstructionScript)

(fn GetTouchDistance
  (bind _returnvalue (Game|GetPlayerController 0))
  (bind (_locationx _locationy) (Class|PlayerController|GetInputTouchState _returnvalue "Touch2"))
  (bind (_locationx_2 _locationy_2) (Class|PlayerController|GetInputTouchState _returnvalue "Touch1"))
  (bind (_locationx_3 _locationy_3) (Game|Player|GetMousePosition _returnvalue))
  (return (Math|Vector2D|Vector2DLength (select (Utilities|Enum|Equal(Enum) (Game|GetPlatformName) "Windows") (Math|Vector2D|MakeVector2D _locationx_3 _locationy_3) (- (Math|Vector2D|MakeVector2D _locationx_2 _locationy_2) (Math|Vector2D|MakeVector2D _locationx _locationy))))))